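; Player controller that handles the game's end-of-match screens for game over and victory.
; On BeginPlay it sets input to game-only.
; ShowGameOverScreen and ShowVictoryScreen each create their widget, add it to the viewport and destroy the controlled pawn.
; Each then switches to UI-only input focused on that widget, with the mouse locked in fullscreen.
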(event `self.ReceiveBeginPlay`
  (`WidgetBlueprintLibrary.SetInputMode_GameOnly` self))

(event `ShowGameOverScreen`
  (bind _returnvalue (`|CreateWidget` "/Game/Blueprints/WBP_GameOver.WBP_GameOver_C"))
  (`UserWidget.AddToViewport` _returnvalue 0)
  (`self.K2_DestroyActor` (`self.K2_GetPawn`))
  (`WidgetBlueprintLibrary.SetInputMode_UIOnlyEx` self _returnvalue "LockInFullscreen"))

(event `ShowVictoryScreen`
  (bind _returnvalue (`|CreateWidget` "/Game/Blueprints/WBP_Victory.WBP_Victory_C"))
  (`UserWidget.AddToViewport` _returnvalue 0)
  (`self.K2_DestroyActor` (`self.K2_GetPawn`))
  (`WidgetBlueprintLibrary.SetInputMode_UIOnlyEx` self _returnvalue "LockInFullscreen"))

(fn `UserConstructionScript`)