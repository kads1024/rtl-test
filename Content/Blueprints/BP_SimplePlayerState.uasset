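; BP_SimplePlayerState is a player state that tracks collected coins and whether the key item has been collected.
; IncrementCoinCount raises the count, copies it to TotalCollectedCoins on BP_SimpleGameMode, and, at or above TargetCoins, tells the level's BP_KeySpawner to spawn the key.
; CollectKeyItem sets the key flag and resets the local coin count, which also starts at zero on BeginPlay.
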(event `self.ReceiveBeginPlay`
  (set `self.CollectedCoins` 0))

(fn `CollectKeyItem`
  (set `self.HasCollectedKeyItem` true)
  (set `self.CollectedCoins` 0))

(fn `IncrementCoinCount`
  (bind _result (`/Engine/EditorBlueprintResources/StandardMacros.IncrementInt` (`self.CollectedCoins`))
    (:`  `
      (bind _asbp_simple_game_mode (cast `/Game/Blueprints/BP_SimpleGameMode` (`GameplayStatics.GetGameMode`)))
      (set `/Game/Blueprints/BP_SimpleGameMode.TotalCollectedCoins` _result _asbp_simple_game_mode)
      (if (>= _result (`self.TargetCoins`))
        (bind _returnvalue (`GameplayStatics.GetActorOfClass` "/Game/Blueprints/BP_KeySpawner.BP_KeySpawner_C"))
        (`/Game/Blueprints/BP_KeySpawner.SpawnKeyItem` _returnvalue)
        (`KismetSystemLibrary.PrintString` "COLLECTED ALL COINS")))))

(fn `UserConstructionScript`)